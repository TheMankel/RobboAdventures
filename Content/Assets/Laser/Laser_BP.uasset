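; Laser hazard actor that dissolves the player's third-person character when it overlaps the collision box.
; BeginPlay starts a looping timer, and ToggleLaser flips the beam's visibility, enabling box collision only while the beam is visible.
; The construction script calls UpdateLaser to set the Laser's BeamEnd parameter from the End component's relative location.
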(event OnComponentBeginOverlap(Box)
  (params (OverlappedComponent :type Primitive%20Component%20Object%20Reference) (OtherActor :type Actor%20Object%20Reference) (OtherComp :type Primitive%20Component%20Object%20Reference) (OtherBodyIndex :type Integer) (bFromSweep :type Boolean) (SweepResult :type Hit%20Result%20Structure%20%28by%20ref%29))
  (if (== OtherActor (Game|GetPlayerCharacter 0))
    (Development|PrintString "Dead")
    (bind _asbp_third_person_character (Utilities|Casting|CastToBP_ThirdPersonCharacter (Game|GetPlayerCharacter 0)))
    (Default|Dissolve _asbp_third_person_character)))

(event Custom|ToggleLaser
  (bind _laser (Variables|Default|GetLaser))
  (Rendering|ToggleVisibility _laser false)
  (Collision|SetCollisionEnabled (Variables|Default|GetBox) (select (Variables|/Script/Engine.SceneComponent|GetbVisible _laser) "QueryAndPhysics" "NoCollision")))

(event EventBeginPlay
  (Utilities|Time|SetTimerbyEvent (EventDispatchers|CreateEvent :!event Custom|ToggleLaser) 2.0 true))

(event Collision|EventActorBeginOverlap
  (params (OtherActor :type Actor%20Object%20Reference)))

(event EventTick
  (params (DeltaSeconds :type Float%20%28single-precision%29)))

(fn ConstructionScript
  (CallFunction|UpdateLaser))

(fn UpdateLaser
  (Effects|Components|ParticleSystem|SetVectorParameter (Variables|Default|GetLaser) "BeamEnd" (Variables|/Script/Engine.SceneComponent|GetRelativeLocation (Variables|Default|GetEnd))))