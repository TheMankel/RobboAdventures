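; Double sliding door Blueprint that opens once enough linked triggers are active.
; On BeginPlay it binds to the Interaction_BP component of each actor in Triggers, and each interaction raises or lowers an active count.
; Reaching TriggersNeeded plays a timeline that slides both panels apart through DoorScript.
; Any deactivation reverses the timeline to close the door, regardless of the remaining count.
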(event Custom|OnInteraction
  (params (InteractionState :type Boolean))
  (if InteractionState
    (bind _result (Math|Integer|IncrementInt (Variables|Default|GetTriggersActive))
      (:%20%20
        (if (>= _result (Variables|Default|GetTriggersNeeded))
          (CallFunction|OpenDoor))))
    (else
      (bind _result_2 (Math|Integer|DecrementInt (Variables|Default|GetTriggersActive))
        (:%20%20
          (Variables|Default|SetTriggersActive (Math|Integer|Max(Integer) _result_2))
          (CallFunction|CloseDoor))))))

(event Custom|OpenDoor
  (bind _doorposition (Timeline|DoorTimeline Play)
    (:Update
      (CallFunction|DoorScript _doorposition))))

(event Custom|CloseDoor
  (bind _doorposition (Timeline|DoorTimeline Reverse)
    (:Update
      (CallFunction|DoorScript _doorposition))))

(event EventBeginPlay
  (if (> (Utilities|Array|Length (Variables|Default|GetTriggers)) 0)
    (for _array_element (Variables|Default|GetTriggers)
      (EventDispatchers|BindEventtoOnInteraction (Actor|GetComponentbyClass _array_element "/Game/Assets/Interaction_BP.Interaction_BP_C") (delegate Custom|OnInteraction)))))

(fn ConstructionScript)

(fn DoorScript
  (params (Position :type Float%20%28double-precision%29))
  (bind _returnvalue (* Position -125.0))
  (Transformation|SetRelativeLocation (Variables|Default|GetDoorLeft) (Math|Vector|MakeVector (+ _returnvalue -5e+01) 0.0 1.5e+02) false false)
  (Transformation|SetRelativeLocation (Variables|Default|GetDoorRight) (Math|Vector|MakeVector (+ (* _returnvalue -1.0) 5e+01) 0.0 1.5e+02) false false))