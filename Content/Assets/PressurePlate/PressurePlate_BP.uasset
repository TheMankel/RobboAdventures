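; Pressure plate Blueprint that starts an interaction while any actor stands on it and stops it once empty.
; Trigger overlap events count overlapping actors, and a DoOnce gate fires the first press only, resetting when the last actor leaves.
; Each state change swaps the Cube's material between blue and default and calls start or stop on the InteractionBP.
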(event OnComponentBeginOverlap(Trigger)
  (params (OverlappedComponent :type Primitive%20Component%20Object%20Reference) (OtherActor :type Actor%20Object%20Reference) (OtherComp :type Primitive%20Component%20Object%20Reference) (OtherBodyIndex :type Integer) (bFromSweep :type Boolean) (SweepResult :type Hit%20Result%20Structure%20%28by%20ref%29))
  (if (>= (Utilities|Array|Length (Collision|GetOverlappingActors (Variables|Default|GetTrigger) "/Script/Engine.Actor" :!class /Script/Engine.PrimitiveComponent)) 1)
    (Utilities|FlowControl|DoOnce false
      (:Completed
        (Rendering|Material|SetMaterial (Variables|Default|GetCube) 0 "/Game/LevelPrototyping/Materials/MI_Solid_Blue.MI_Solid_Blue")
        (Default|StartInteraction (Variables|Default|GetInteraction_BP))))))

(event OnComponentEndOverlap(Trigger)
  (params (OverlappedComponent :type Primitive%20Component%20Object%20Reference) (OtherActor :type Actor%20Object%20Reference) (OtherComp :type Primitive%20Component%20Object%20Reference) (OtherBodyIndex :type Integer))
  (bind _interaction_bp (Variables|Default|GetInteraction_BP))
  (if (== (Utilities|Array|Length (Collision|GetOverlappingActors (Variables|Default|GetTrigger) "/Script/Engine.Actor" :!class /Script/Engine.PrimitiveComponent)) 0)
    (Utilities|FlowControl|Sequence
      (:then_0
        (Utilities|FlowControl|DoOnce false) ; enters at Reset
      )
      (:then_1
        (Rendering|Material|SetMaterial (Variables|Default|GetCube) 0 "/Game/LevelPrototyping/Materials/M_Solid.M_Solid")
        (Default|StopInteraction _interaction_bp)))))

(fn ConstructionScript)