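; TrapDoor_BP is a two-panel trap door that swings open on overlap once enough linked triggers have armed it.
; BeginPlay binds each Triggers entry's Interaction_BP event to an active-trigger count, which sets Opened at TriggersNeeded and never clears it.
; Overlapping the Trigger component while Opened plays TrapTimeline, whose value TrapScript uses to pitch FrameLeft and FrameRight in opposite directions.
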(event OnComponentBeginOverlap(Trigger)
  (params (OverlappedComponent :type Primitive%20Component%20Object%20Reference) (OtherActor :type Actor%20Object%20Reference) (OtherComp :type Primitive%20Component%20Object%20Reference) (OtherBodyIndex :type Integer) (bFromSweep :type Boolean) (SweepResult :type Hit%20Result%20Structure%20%28by%20ref%29))
  (if (Variables|Default|GetOpened)
    (bind _trapposition (Timeline|TrapTimeline Play)
      (:Update
        (CallFunction|TrapScript _trapposition)))))

(event Custom|OnInteraction
  (params (InteractionState :type Boolean))
  (if InteractionState
    (bind _result (Math|Integer|IncrementInt (Variables|Default|GetTriggersActive))
      (:%20%20
        (if (>= _result (Variables|Default|GetTriggersNeeded))
          (Variables|Default|SetOpened true))))
    (else
      (bind _result_2 (Math|Integer|DecrementInt (Variables|Default|GetTriggersActive))
        (:%20%20
          (Variables|Default|SetTriggersActive (Math|Integer|Max(Integer) _result_2)))))))

(event EventBeginPlay
  (if (> (Utilities|Array|Length (Variables|Default|GetTriggers)) 0)
    (for _array_element (Variables|Default|GetTriggers)
      (EventDispatchers|BindEventtoOnInteraction (Actor|GetComponentbyClass _array_element "/Game/Assets/Interaction_BP.Interaction_BP_C") (delegate Custom|OnInteraction)))))

(fn ConstructionScript)

(fn TrapScript
  (params (Rotation :type Float%20%28double-precision%29))
  (bind _returnvalue (* Rotation -9e+01))
  (Transformation|SetRelativeRotation (Variables|Default|GetFrameLeft) (Math|Rotator|MakeRotator 0.0 _returnvalue 0.0) false false)
  (Transformation|SetRelativeRotation (Variables|Default|GetFrameRight) (Math|Rotator|MakeRotator 0.0 (* _returnvalue -1.0) 0.0) false false))