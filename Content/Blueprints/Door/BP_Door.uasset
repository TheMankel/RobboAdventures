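; BP_Door is a double sliding door that opens when enough linked trigger actors are active.
; It binds to each trigger's BP_Interaction event, counts activations against TriggersNeeded, and closes on any deactivation.
; A timeline plays or reverses to slide both panels apart or together along relative X via DoorScript.
; The construction script tints linked BP_Key triggers and both panels with a shared Color.
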(event Custom|OnInteraction
  (params (InteractionState :type Boolean))
  (if InteractionState
    (bind _result (Math|Integer|IncrementInt (Variables|Default|GetTriggersActive))
      (:%20%20
        (if (>= _result (Variables|Default|GetTriggersNeeded))
          (CallFunction|OpenDoor))))
    (else
      (bind _result_2 (Math|Integer|DecrementInt (Variables|Default|GetTriggersActive))
        (:%20%20
          (Variables|Default|SetTriggersActive (Math|Integer|Max(Integer) _result_2))
          (CallFunction|CloseDoor))))))

(event Custom|OpenDoor
  (bind _doorposition (Timeline|DoorTimeline Play)
    (:Update
      (CallFunction|DoorScript _doorposition))))

(event Custom|CloseDoor
  (bind _doorposition (Timeline|DoorTimeline Reverse)
    (:Update
      (CallFunction|DoorScript _doorposition))))

(event EventBeginPlay
  (if (> (Utilities|Array|Length (Variables|Default|GetTriggers)) 0)
    (for _array_element (Variables|Default|GetTriggers)
      (EventDispatchers|BindEventtoOnInteraction (Actor|GetComponentbyClass _array_element "/Game/Blueprints/BP_Interaction.BP_Interaction_C") (delegate Custom|OnInteraction)))))

(fn ConstructionScript
  (bind _color (Variables|Default|GetColor))
  (if (> (Utilities|Array|Length (Variables|Default|GetTriggers)) 0)
    (for _array_element (Variables|Default|GetTriggers)
      (bind _asbp_key (Utilities|Casting|CastToBP_Key _array_element))
      (Rendering|Material|SetVectorParameterValueonMaterials (Variables|/Game/Blueprints/Key/BP_Key.BP_Key_C|GetKey _asbp_key) "Tint" _color)
      (Rendering|Material|SetVectorParameterValueonMaterials (Variables|Default|GetDoorLeft) "Tint" _color)
      (Rendering|Material|SetVectorParameterValueonMaterials (Variables|Default|GetDoorRight) "Tint" _color))))

(fn DoorScript
  (params (Position :type Float%20%28double-precision%29))
  (bind _returnvalue (* Position 175.0))
  (bind _doorright (Variables|Default|GetDoorRight))
  (bind _doorleft (Variables|Default|GetDoorLeft))
  (bind _relativelocation (Variables|/Script/Engine.SceneComponent|GetRelativeLocation _doorleft))
  (bind _relativelocation_2 (Variables|/Script/Engine.SceneComponent|GetRelativeLocation _doorright))
  (Transformation|SetRelativeLocation _doorright (Math|Vector|MakeVector _returnvalue (.y _relativelocation_2) (.z _relativelocation_2)) false false)
  (Transformation|SetRelativeLocation _doorleft (Math|Vector|MakeVector (* _returnvalue -1.0) (.y _relativelocation) (.z _relativelocation)) false false))