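; BP_Projectile is a projectile actor that damages characters and pushes physics objects it hits.
; On Hit, a BP_ThirdPersonCharacter takes fixed damage with the projectile as damage causer, and the projectile is destroyed.
; For any other valid component, it applies a velocity-scaled impulse at its own location if that component simulates physics, then destroys itself either way.
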(event Collision|EventHit
  (params (MyComp :type Primitive%20Component%20Object%20Reference) (Other :type Actor%20Object%20Reference) (OtherComp :type Primitive%20Component%20Object%20Reference) (bSelfMoved :type Boolean) (HitLocation :type Vector :default "0, 0, 0") (HitNormal :type Vector :default "0, 0, 0") (NormalImpulse :type Vector :default "0, 0, 0") (Hit :type Hit%20Result%20Structure%20%28by%20ref%29))
  (bind _asbp_third_person_character (Utilities|Casting|CastToBP_ThirdPersonCharacter Other)
    (:then
      (Game|Damage|ApplyDamage _asbp_third_person_character 1e+02 0 self)
      (Actor|DestroyActor))
    (:CastFailed
      (Utilities|IsValid OtherComp
        (:Is%20Valid
          (if (Physics|IsSimulatingPhysics OtherComp "None")
            (Physics|AddImpulseatLocation OtherComp (* (Transformation|GetVelocity) 1e+02) (Transformation|GetActorLocation) "None")
            (Actor|DestroyActor)
            (else
              (Actor|DestroyActor))))))))

(fn ConstructionScript)