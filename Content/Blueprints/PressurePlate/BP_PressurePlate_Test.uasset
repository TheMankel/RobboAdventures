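; BP_PressurePlate_Test is a pressure plate actor that starts and stops an interaction through its BPInteraction member.
; When an Actor overlaps the Trigger, a DoOnce gate lights both platform meshes via the PlatformActive material parameter and calls StartInteraction.
; When the last overlapping Actor leaves, it resets the gate, clears the parameter and calls StopInteraction, so additional occupants do not retrigger it.
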(event OnComponentBeginOverlap(Trigger)
  (params (OverlappedComponent :type Primitive%20Component%20Object%20Reference) (OtherActor :type Actor%20Object%20Reference) (OtherComp :type Primitive%20Component%20Object%20Reference) (OtherBodyIndex :type Integer) (bFromSweep :type Boolean) (SweepResult :type Hit%20Result%20Structure%20%28by%20ref%29))
  (if (>= (Utilities|Array|Length (Collision|GetOverlappingActors (Variables|Default|GetTrigger) "/Script/Engine.Actor" :!class /Script/Engine.PrimitiveComponent)) 1)
    (Utilities|FlowControl|DoOnce false
      (:Completed
        (Rendering|Material|SetScalarParameterValueonMaterials (Variables|Default|GetSM_Platform_Right) "PlatformActive" 1.0)
        (Default|StartInteraction (Variables|Default|GetBP_Interaction))))))

(event OnComponentEndOverlap(Trigger)
  (params (OverlappedComponent :type Primitive%20Component%20Object%20Reference) (OtherActor :type Actor%20Object%20Reference) (OtherComp :type Primitive%20Component%20Object%20Reference) (OtherBodyIndex :type Integer))
  (bind _bp_interaction (Variables|Default|GetBP_Interaction))
  (if (== (Utilities|Array|Length (Collision|GetOverlappingActors (Variables|Default|GetTrigger) "/Script/Engine.Actor" :!class /Script/Engine.PrimitiveComponent)) 0)
    (Utilities|FlowControl|Sequence
      (:then_0
        (Utilities|FlowControl|DoOnce false) ; enters at Reset
      )
      (:then_1
        (Rendering|Material|SetScalarParameterValueonMaterials (Variables|Default|GetSM_Platform_Right) "PlatformActive" 0.0)
        (Default|StopInteraction _bp_interaction)))))

(event EventBeginPlay
  (|CallParentFunction) ; This node is disabled and will not be called.\nDrag off pins to build functionality.
)

(event Collision|EventActorBeginOverlap
  (params (OtherActor :type Actor%20Object%20Reference))
  (|CallParentFunction OtherActor) ; This node is disabled and will not be called.\nDrag off pins to build functionality.
)

(event EventTick
  (params (DeltaSeconds :type Float%20%28single-precision%29))
  (|CallParentFunction DeltaSeconds) ; This node is disabled and will not be called.\nDrag off pins to build functionality.
)

(fn ConstructionScript
  (|CallParentFunction))