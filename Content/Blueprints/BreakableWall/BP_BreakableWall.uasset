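; BP_BreakableWall is a destructible wall that breaks when it takes any damage.
; Break spawns a short-lived BP_Damage actor at the TriggerBox transform, alongside a Geometry Collection for the debris.
; After a short delay, a timeline drives the debris material's Alpha Threshold parameter to fade the pieces out, then destroys the wall.
; Debug prints report the damage causer and the break.
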(event Custom|Break
  (bind _returnvalue (Game|SpawnActorfromClass "/Game/Blueprints/BreakableWall/BP_Damage.BP_Damage_C" (Transformation|GetWorldTransform (Variables|Default|GetTriggerBox)) "Undefined" 0 0))
  (Actor|SetLifeSpan _returnvalue 0.5)
  (Development|PrintString "Break")
  (Utilities|FlowControl|Delay 1.0)
  (bind _fade_value (Timeline|Fade%20Debris Play)
    (:Update
      (Rendering|Material|SetScalarParameterValueonMaterials (Variables|Default|GetGeometryCollectionComponent) "Alpha Threshold" _fade_value))
    (:Finished
      (Actor|DestroyActor))))

(event Game|Damage|EventAnyDamage
  (params (Damage :type Float%20%28single-precision%29) (DamageType :type Damage%20Type%20Object%20Reference) (InstigatedBy :type Controller%20Object%20Reference) (DamageCauser :type Actor%20Object%20Reference))
  (Development|PrintString (Utilities|GetDisplayName DamageCauser))
  (CallFunction|Break))

(fn ConstructionScript)