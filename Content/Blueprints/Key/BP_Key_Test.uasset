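; BP_Key_Test is a key pickup actor, named as a test, that the third-person player character or a test bot collects by touching it.
; When either one overlaps its collision sphere, it starts an interaction through its BPInteraction reference, prints a pickup message and destroys itself.
; Both cast checks share that same pickup sequence, and any other actor is ignored.
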(event OnComponentBeginOverlap(CollisionSphere)
  (params (OverlappedComponent :type Primitive%20Component%20Object%20Reference) (OtherActor :type Actor%20Object%20Reference) (OtherComp :type Primitive%20Component%20Object%20Reference) (OtherBodyIndex :type Integer) (bFromSweep :type Boolean) (SweepResult :type Hit%20Result%20Structure%20%28by%20ref%29))
  (Utilities|Casting|CastToBP_ThirdPersonCharacter OtherActor
    (:then
      _)
    (:CastFailed
      (Utilities|Casting|CastToBP_TestBot OtherActor)))
  (Default|StartInteraction (Variables|Default|GetBP_Interaction))
  (Development|PrintString "Pick up")
  (Actor|DestroyActor))

(event EventBeginPlay
  (|CallParentFunction) ; This node is disabled and will not be called.\nDrag off pins to build functionality.
)

(event Collision|EventActorBeginOverlap
  (params (OtherActor :type Actor%20Object%20Reference))
  (|CallParentFunction OtherActor) ; This node is disabled and will not be called.\nDrag off pins to build functionality.
)

(event EventTick
  (params (DeltaSeconds :type Float%20%28single-precision%29))
  (|CallParentFunction DeltaSeconds) ; This node is disabled and will not be called.\nDrag off pins to build functionality.
)

(fn ConstructionScript
  (|CallParentFunction))