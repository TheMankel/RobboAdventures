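; BP_Enemy is an AI enemy character with a gun, a spline movement path and sight-based detection of the player.
; On begin play it sets walk speed and detaches the path so it stays fixed in the world.
; Sight updates on the third-person character set or clear the blackboard's TargetActor.
; The Shoot event spawns a projectile near the gun along the actor's rotation and plays a rifle fire montage.
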(event OnTargetPerceptionUpdated(AIPerception)
  (params (Actor :type Actor%20Object%20Reference) (Stimulus :type AI%20Stimulus%20Structure))
  (CallFunction|HandleSightSense Actor Stimulus))

(event Custom|Shoot
  (bind _returnvalue (Transformation|GetActorRotation))
  (Game|SpawnActorfromClass "/Game/Blueprints/Projectile/BP_Projectile.BP_Projectile_C" (Math|Transform|MakeTransform (+ (Transformation|GetSocketLocation (Variables|Default|GetSK_Gun) "None") (Math|Vector|RotateVector "100.000000,0.000000,-10.000000" _returnvalue)) _returnvalue) "Undefined" 0 0)
  (Animation|Montage|MontagePlay (Components|SkeletalMesh|GetAnimInstance (Variables|Character|GetMesh)) "/Game/Characters/EnemyBot/Animations/Enemy/MM_Rifle_Fire_Montage.MM_Rifle_Fire_Montage" 1.0 "MontageLength" 0.0 true))

(event EventBeginPlay
  (Variables|/Script/Engine.CharacterMovementComponent|SetMaxWalkSpeed (Variables|Character|GetCharacterMovement) (Variables|Default|GetWalkSpeed))
  (Transformation|DetachFromComponent (Variables|Default|GetMovementPath) "KeepWorld" "KeepWorld" "KeepWorld" true))

(fn ConstructionScript
  (if (Variables|Default|GetPathIsClosedLoop)
    (Spline|SetClosedLoop (Variables|Default|GetMovementPath) true true)))

(fn HandleSightSense
  (params (Actor :type Actor%20Object%20Reference) (Stimulus :type AI%20Stimulus%20Structure))
  (bind _returnvalue (Class|AIPerceptionSystem|GetSenseClassforStimulus Stimulus))
  (if (== _returnvalue "/Script/AIModule.AISense_Sight")
    (bind _asbp_third_person_character (Utilities|Casting|CastToBP_ThirdPersonCharacter Actor)
      (:then
        (AI|Components|Blackboard|SetValueasObject (AI|GetBlackboard 0) (Utilities|Name|MakeLiteralName "TargetActor") (select (.bsuccessfullysensed Stimulus) _asbp_third_person_character 0)))
      (:CastFailed
        (return)))
    (else
      (return))))